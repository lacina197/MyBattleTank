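; Player-controlled tank Blueprint that wires up aiming camera controls and firing.
; On BeginPlay it registers its barrel and turret components through SetBarrelReference and SetTurretReference.
; Azimuth input yaws a gimbal and elevation input pitches the spring arm, splitting camera rotation across two components.
; The fire action calls Fire, while the left and right track throttle axes are still empty stubs.
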(event `self.ReceiveBeginPlay`
  (`self.SetBarrelReference` (`self.Barel`))
  (`self.SetTurretReference` (`self.Turret`)))

(event `InputAxis|AimAzimuth`
  (params (AxisValue :type "Float (single-precision)"))
  ;[1 1 1] Camera Input Binding
  (`SceneComponent.K2_AddLocalRotation` (`self.Azimuth Gimbal`) (`KismetMathLibrary.MakeRotator` 0.0 0.0 AxisValue) false false))

(event `InputAxis|Left Track Throttle`
  (params (AxisValue :type "Float (single-precision)")))

(event `InputAxis|Right Track Throttle`
  (params (AxisValue :type "Float (single-precision)")))

(event `InputAxis|AimElevation`
  (params (AxisValue :type "Float (single-precision)"))
  ;[1 1 1] Camera Input Binding
  (`SceneComponent.K2_AddLocalRotation` (`self.SpringArm`) (`KismetMathLibrary.MakeRotator` 0.0 AxisValue) false false))

(event `InputAction|Fire`
  (params (Key :type "Key Structure"))
  (:`Pressed`
    (`self.Fire`)))

(fn `UserConstructionScript`)